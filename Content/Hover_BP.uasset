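; Hover Blueprint that counteracts gravity on its static mesh while a surface is within a set Height below it.
; Each Tick it casts a debug-drawn Visibility line trace straight down from the mesh's location.
; On a hit, it applies a constant upward force of mass times gravitational acceleration, with no scaling by distance or damping.
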(event `self.ReceiveTick`
  (params (DeltaSeconds :type "Float (single-precision)"))
  (bind _returnvalue (`SceneComponent.K2_GetComponentLocation` (`self.StaticMeshComponent`)))
  (bind (_outhit _returnvalue_2) (`KismetSystemLibrary.LineTraceSingle` :`Start` _returnvalue :`End` (+ _returnvalue (`KismetMathLibrary.MakeVector` 0.0 0.0 (* (`self.Height`) -1.0))) :`TraceChannel` "TraceTypeQuery1" :`DrawDebugType` "ForOneFrame"))
  (if _returnvalue_2
    (`PrimitiveComponent.AddForce` (`self.StaticMeshComponent`) (* (`KismetMathLibrary.MakeVector` 0.0 0.0 980.0) (`PrimitiveComponent.GetMass` (`self.StaticMeshComponent`))) "None" false)))

(fn `UserConstructionScript`)