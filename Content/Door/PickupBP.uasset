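; PickupBP is a pickup actor that can be picked up and dropped, and reports a weight based on its state.
; Pickup and Dropped events toggle a picked-up flag and print the object's name, and Destroyed prints a debug message.
; GetWeight returns the static mesh's mass only when the object is not held and nearly stationary, checked by squared velocity, and zero otherwise.
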(event `self.ReceiveBeginPlay`)

(event `Pickup`
  (set `self.PickedUpFlag` true)
  (`KismetSystemLibrary.PrintString` (`KismetTextLibrary.Conv_TextToString` (`|FormatText` "Picked up {Me}" (`KismetTextLibrary.Conv_StringToText` (`KismetSystemLibrary.GetDisplayName` self))))))

(event `Dropped`
  (set `self.PickedUpFlag` false)
  (`KismetSystemLibrary.PrintString` (`KismetTextLibrary.Conv_TextToString` (`|FormatText` "Dropped {Me}" (`KismetTextLibrary.Conv_StringToText` (`KismetSystemLibrary.GetDisplayName` self))))))

(event `self.ReceiveDestroyed`
  (`KismetSystemLibrary.PrintString` "Dead"))

(fn `getWeight`
  (returns (Return :type "Float (double-precision)"))
  ;[1 1 1] Is it picked up?
  (bind _result (`self.IsPickedUp`))
  (if _result
    _
    (elif (<= (`KismetMathLibrary.VSizeSquared` (`self.GetVelocity`)) 0.1)
      ;[1 1 1] When dropped and static get weigh
      (return (`PrimitiveComponent.GetMass` (`self.StaticMeshComponent`)))
      (else
        _)))
  ;[1 1 1] If moving or still picked up, dont count weight
  (return 0.0))

(fn `IsPickedUp`
  (returns (Result :type Boolean))
  (return (`self.PickedUpFlag`)))

(fn `UserConstructionScript`)