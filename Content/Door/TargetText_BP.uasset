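; TargetText_BP is a shootable text target that shows "Trigger {ID}" and acts as a switch for a linked door.
; On BeginPlay it sets its label, sizes the box collider to the text's bounds, stores the original colour and registers via LinkTarget on DoorRef.
; A FirstPersonProjectile overlap calls SwitchHit on the door.
; UpdateResult flashes the text green or red for correct or wrong, restoring the colour after a delay.
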(event `self.ReceiveBeginPlay`
  ;[1 1 1] Debug Change Text to Trigger ID
  (`TextRenderComponent.K2_SetText` (`self.TextRender`) (`|FormatText` "Trigger {ID}" (`self.ID`)))
  ;[1 1 1] Adjust Box size to new text size, note size = 2 x Exent, so needs to halve
  (`BoxComponent.SetBoxExtent` (`self.Collider`) (/ (`KismetMathLibrary.MakeVector` 32.0 (.y (`TextRenderComponent.GetTextLocalSize` (`self.TextRender`))) (.z (`TextRenderComponent.GetTextLocalSize` (`self.TextRender`)))) 2.0) true)
  ;[1 1 1] Remember original colour
  (bind _output_get (set `self.DefaultColour` (`TextRenderComponent.TextRenderColor` (`self.TextRender`))))
  ;[1 1 1] Tell door about us
  (`/Game/Door/OpeningDoor_BP.LinkTarget` (`self.DoorRef`) null))

(event `self.ReceiveActorBeginOverlap`
  (params (OtherActor :type "Actor Object Reference"))
  (bind _doorref (`self.DoorRef`))
  ;[1 1 1] Hit By bullet
  (cast `/Game/FirstPerson/FirstPersonProjectile` OtherActor)
  ;[1 1 1] Signal door
  (if (`KismetSystemLibrary.IsValid` _doorref)
    (`/Game/Door/OpeningDoor_BP.SwitchHit` _doorref self)
    (else
      ;[1 1 1] Check DoorRef OK
      (`KismetSystemLibrary.PrintString` "DoorRef not set"))))

(event `UpdateResult`
  (params (Correct :type Boolean))
  (bind _textrender (`self.TextRender`))
  ;[1 1 1] Pick colour if hit
  (`TextRenderComponent.SetTextRenderColor` _textrender (select `bool` Correct :`false` (`KismetMathLibrary.Conv_LinearColorToColor` (`KismetMathLibrary.MakeColor` 1.0)) :`true` (`KismetMathLibrary.Conv_LinearColorToColor` (`KismetMathLibrary.MakeColor` 0.0 1.0))))
  (`KismetSystemLibrary.Delay` 2.0)
  (`TextRenderComponent.SetTextRenderColor` _textrender (stale `self.ReceiveBeginPlay` _output_get)))

(fn `UserConstructionScript`)