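; Hinged door that opens when its linked switch targets are hit in ID order, then auto-closes.
; Targets register through LinkTarget to set the sequence length; SwitchHit reports each result back to the target, advancing on a match and resetting otherwise.
; A timeline rotates the hinge by a configurable angle with a click sound, while a busy flag blocks overlapping commands and Tick counts down the close timer.
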(event `self.ReceiveBeginPlay`
  ;[1 1 1] Set Inital door state
  (`self.SetDoorTime` (`self.isDoorOpen`)))

(event `self.ReceiveTick`
  (params (DeltaSeconds :type "Float (single-precision)"))
  (bind _closetimer (`self.CloseTimer`))
  ;[1 0.6355 0.4857] Check if autoclose needed
  (if (`self.isDoorOpen`)
    ;[1 0.6355 0.4857] Update Autoclose time, and clamp at 0 if done
    (if (`KismetMathLibrary.NearlyEqual_FloatFloat` _closetimer)
      (set `self.CloseTimer` 0.0)
      (else
        (bind _output_get (set `self.CloseTimer` (- _closetimer DeltaSeconds)))
        (if (<= _output_get 0.0)
          (`self.SetDoorState` false))))))

(event `SetDoorState`
  (params (setOpen :type Boolean :default true) (AutoClose :type "Float (double-precision)"))
  (bind _isdooropen (`self.isDoorOpen`))
  (bind _dooraction (`self.DoorAction`))
  ;[1 1 1] Set door open or closed, but only action if needed
  ;;[1 0.4498 0.7466] If door busy ignore command
  (if (`self.isDoorBusy`)
    _
    (elif setOpen
      (if (not _isdooropen)
        ;[1 1 1] Set Door busy
        (set `self.isDoorBusy` true)
        ;[1 1 1] Door Time Line
        (bind (_direction _anglemultiplier) (`Timeline|DoorAction` :`NewTime` (`KismetMathLibrary.SelectFloat` (`TimelineComponent.GetTimelineLength` (`self.DoorAction`)) 0.0 (stale `SetDoorTime` setOpen)) :!label _label)
          (:`Update`
            ;[1 0.3771 0.8036] Open door by rotating hinge pivot
            (`SceneComponent.K2_SetRelativeRotation` (`self.Door`) (`KismetMathLibrary.MakeRotator` 0.0 0.0 (* _anglemultiplier (`self.OpenAngle`))) false false))
          (:`Finished`
            ;[1 1 1] Set Open flag once motion complete, also set autoclose time
            (set `self.isDoorOpen` (>= (`TimelineComponent.GetPlaybackPosition` _dooraction) (/ (`TimelineComponent.GetTimelineLength` _dooraction) 2.0)))
            (set `self.CloseTimer` AutoClose)
            ;;[1 0.3917 0.7912] Door no longer busy
            (set `self.isDoorBusy` false))
          (:`Triggers`
            ;[0.2109 1 0.1548] Door clunk
            (`AudioComponent.Play` (`self.DoorClick`) 0.0))))
      (elif _isdooropen
        (set `self.isDoorBusy` true)
        (goto _label :!via `Reverse`)))))

(event `SetDoorTime`
  (params (setOpen :type Boolean))
  ;[1 1 1] Set Initial door state
  (goto _label :!via `SetNewTime`))

(event `SwitchHit`
  (params (TargetRef :type "/Game/Door/TargetText_BP Object Reference"))
  (bind _nextswitch (`self.NextSwitch`))
  (bind _id (`/Game/Door/TargetText_BP.ID` TargetRef))
  (bind _returnvalue (== _id _nextswitch))
  ;[1 1 1] Programable door lock state machine
  ;;[1 1 1] Switch hit
  ;;[1 1 1] DebugText
  (`KismetSystemLibrary.PrintString` (`KismetTextLibrary.Conv_TextToString` (`|FormatText` "Switch {ID} Hit Expected {Next}" _id _nextswitch)))
  (`/Game/Door/TargetText_BP.UpdateResult` TargetRef _returnvalue)
  ;;[0.4027 0.5334 1] Is it the switch we are expecting?
  (if _returnvalue
    ;;[1 0.3453 0.5105] Set next switch & check if at the end of sequence
    (bind _result (`/Engine/EditorBlueprintResources/StandardMacros.IncrementInt` (`self.NextSwitch`))
      (:`  `
        (if (== _result (+ (`self.SwitchCount`) 1))
          ;;[1 1 1] Open Door
          (`self.SetDoorState` true 5.0)
          ;;[1 0.8301 0.0429] Reset Switch
          (set `self.NextSwitch` 1 :!label _label_2)
          (`KismetSystemLibrary.PrintString` "Sequence Reset"))))
    (else
      (goto _label_2))))

(event `LinkTarget`
  (params (LinkMe :type "/Game/Door/TargetText_BP Object Reference"))
  (bind _targetarray (`self.TargetArray`))
  ;[1 1 1] Have all the targets report in, and store them, also update switch count
  (`KismetArrayLibrary.Array_Add` _targetarray LinkMe)
  (bind _output_get (set `self.SwitchCount` (`KismetArrayLibrary.Array_Length` _targetarray)))
  (`KismetSystemLibrary.PrintString` (`KismetTextLibrary.Conv_TextToString` (`|FormatText` "{Door} {Count} Targets" (`KismetTextLibrary.Conv_StringToText` (`KismetSystemLibrary.GetDisplayName` self)) _output_get))))

(fn `UserConstructionScript`)