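; ScalesBP is a weighing scale that opens a linked door when the weight on it reaches a required threshold.
; On BeginPlay and whenever a Tick countdown expires, it sums the weights of pickups and player characters overlapping its collider.
; It then displays the total in kg, passes the open state and an auto-close time to DoorRef, and recolours the text by threshold.
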(event `self.ReceiveBeginPlay`
  (bind _doorref (`self.DoorRef`))
  (bind _weight (`self.Weight`))
  (bind _overlappingactors (`PrimitiveComponent.GetOverlappingActors` (`self.Collider`) null))
  (bind _returnvalue (>= _weight (`self.OpenWeight`)))
  ;[1 1 1] Trigger inital weighing
  (set `self.WeighCountDown` (`self.WeighTime`))
  ;[1 1 1] Scale Timeout, Reset Weight
  (set `self.Weight` 0.0 :!label _label)
  ;[1 1 1] Check if we have stuff on scales
  (if (> (`KismetArrayLibrary.Array_Length` _overlappingactors) 0)
    ;[1 1 1] Weigh stuff on scales, could be pickup or player, so deal with both
    (for _array_element _overlappingactors
      (bind _aspickup_bp (cast `/Game/Door/PickupBP` _array_element)
        (:`then`
          (bind _return (`/Game/Door/PickupBP.getWeight` _aspickup_bp))
          (set `self.Weight` (+ _return (`self.Weight`))))
        (:`CastFailed`
          ;[1 1 1] Weigh player if they step on scale
          (bind _asfirst_person_character (cast `/Game/FirstPerson/FirstPersonCharacter` _array_element))
          (bind _weight_2 (`/Game/FirstPerson/FirstPersonCharacter.GetWeight` _asfirst_person_character))
          (set `self.Weight` (+ _weight_2 (`self.Weight`)))))))
  ;[1 1 1] Split Execution to update text and deal with door open
  (`|ExecutionSequence`
    (:`then_0`
      ;[1 1 1] Show weight on scale
      (`TextRenderComponent.K2_SetText` (`self.WeightText`) (`|FormatText` "{Weight} kg" _weight)))
    (:`then_1`
      ;[1 1 1] Tell Door to open, if we have correct weight
      (if (`KismetSystemLibrary.IsValid` _doorref)
        (`/Game/Door/OpeningDoor_BP.SetDoorState` _doorref _returnvalue 10.0)
        ;[1 1 1] Set scale text colour
        (`TextRenderComponent.SetTextRenderColor` (`self.WeightText`) (select `bool` _returnvalue :`false` (`self.TooLow`) :`true` (`self.OK`)))
        (else
          ;;[1 1 1] Debug helper, if we forget to link DoorRef
          (`KismetSystemLibrary.PrintString` "Missing Door Ref"))))))

(event `self.ReceiveTick`
  (params (DeltaSeconds :type "Float (single-precision)"))
  ;[1 1 1] Scale Timeout, Reset Weight
  (bind _output_get (set `self.WeighCountDown` (- (`self.WeighCountDown`) DeltaSeconds)))
  (if (< _output_get 0.0)
    (set `self.WeighCountDown` (`self.WeighTime`))
    (goto _label)))

(fn `UserConstructionScript`)