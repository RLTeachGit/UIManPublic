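; Actor component that makes its owner's static mesh hover above surfaces using physics forces.
; On BeginPlay it scales normalized offsets by the mesh's bounds and world scale to build hover points.
; Each Tick it rotates the points with the mesh and traces down by the hover height.
; Hits apply upward spring-like force at that point, scaled by proximity, mass and gravity, divided among all points, without damping.
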(event `self.ReceiveBeginPlay`
  (bind _returnvalue (`self.GetOwner`))
  (bind (_min _max) (`StaticMeshComponent.GetLocalBounds` (`self.StaticMesh`)))
  (bind _x (.x _min))
  (bind _y (.y _min))
  (bind _x_2 (.x _max))
  (bind _y_2 (.y _max))
  (set `self.Parent` _returnvalue)
  (set `self.StaticMesh` (`Actor.GetComponentByClass` _returnvalue "/Script/Engine.StaticMeshComponent"))
  (bind _output_get (set `self.ExtendX` (* (/ (- (`KismetMathLibrary.FMax` _x _x_2) (`KismetMathLibrary.FMin` _x _x_2)) 2.0) (.x (`SceneComponent.K2_GetComponentScale` (`self.StaticMesh`))))))
  (bind _output_get_2 (set `self.ExtendY` (* (/ (- (`KismetMathLibrary.FMax` _y _y_2) (`KismetMathLibrary.FMin` _y _y_2)) 2.0) (.y (`SceneComponent.K2_GetComponentScale` (`self.StaticMesh`))))))
  (for (_array_element _array_index) (`self.Offsets`)
    (`KismetArrayLibrary.Array_Set` (`self.Points`) _array_index (`KismetMathLibrary.MakeVector` (* (.x _array_element) _output_get) (* (.y _array_element) _output_get_2) (/ (+ (.z _min) (.z _max)) 2.0)) true))
  (`KismetSystemLibrary.PrintString` "Hover Active"))

(event `self.ReceiveTick`
  (params (DeltaSeconds :type "Float (single-precision)"))
  (bind _staticmesh (`self.StaticMesh`))
  (bind _height (`self.Height`))
  (for _array_element (`self.Points`)
    (bind _returnvalue (+ (`KismetMathLibrary.GreaterGreater_VectorRotator` _array_element (`SceneComponent.K2_GetComponentRotation` _staticmesh)) (`SceneComponent.K2_GetComponentLocation` _staticmesh)))
    (bind (_outhit _returnvalue_2) (`KismetSystemLibrary.LineTraceSingle` :`Start` _returnvalue :`End` (- _returnvalue (`KismetMathLibrary.MakeVector` 0.0 0.0 (`self.Height`))) :`TraceChannel` "TraceTypeQuery1" :`DrawDebugType` (`self.Debug`)))
    (if _returnvalue_2
      (`PrimitiveComponent.AddForceAtLocation` (`self.StaticMesh`) (`KismetMathLibrary.MakeVector` 0.0 0.0 (/ (* (`PrimitiveComponent.GetMass` (`self.StaticMesh`)) (`self.Gravity`) (`self.Boost`) (`KismetMathLibrary.FClamp` (* (/ (- _height (.z (- _returnvalue (`.Location` (`GameplayStatics.BreakHitResult` _outhit))))) _height) (`self.Speed`)))) (`KismetMathLibrary.Conv_IntToDouble` (`KismetArrayLibrary.Array_Length` (`self.Points`))))) _returnvalue "None"))))